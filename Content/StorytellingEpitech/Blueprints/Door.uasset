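; Sliding double-door actor that opens and closes when triggered or untriggered through the Triggerable interface.
; The construction script records both panels' closed relative locations.
; Trigger events set the Open flag and play the same sound at the door on either change.
; Tick continuously eases each panel with VInterpTo toward its closed location or an opposite X offset from it, depending on that flag.
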(event `self.ReceiveBeginPlay`)

(event `self.ReceiveTick`
  (params (DeltaSeconds :type "Float (single-precision)"))
  (bind _leftclosedlocation (`self.LeftClosedLocation`))
  (bind _rightclosedlocation (`self.RightClosedLocation`))
  (`SceneComponent.K2_SetRelativeLocation` (`self.LeftDoor`) (`KismetMathLibrary.VInterpTo` (`SceneComponent.RelativeLocation` (`self.LeftDoor`)) (`KismetMathLibrary.SelectVector` (- _leftclosedlocation (`KismetMathLibrary.MakeVector` (`self.DoorOpenOffset`))) _leftclosedlocation (`self.Open`)) DeltaSeconds 5.0) false false)
  (`SceneComponent.K2_SetRelativeLocation` (`self.RightDoor`) (`KismetMathLibrary.VInterpTo` (`SceneComponent.RelativeLocation` (`self.RightDoor`)) (`KismetMathLibrary.SelectVector` (+ _rightclosedlocation (`KismetMathLibrary.MakeVector` (`self.DoorOpenOffset`))) _rightclosedlocation (`self.Open`)) DeltaSeconds 5.0) false false))

(event `self.Triggerable.OnTrigger`
  (params (Instigator :type "Actor Object Reference") (`Instigator Component` :type "ActorComponent Object Reference"))
  (set `self.Open` true)
  (`GameplayStatics.PlaySoundAtLocation` "/Game/ThirdPerson/Sounds/SF-fermport.SF-fermport" (`self.K2_GetActorLocation`) (struct) 1.0 1.0 0.0 null null null null :!label _label))

(event `self.Triggerable.OnUntrigger`
  (params (Instigator :type "Actor Object Reference") (`Instigator Component` :type "ActorComponent Object Reference"))
  (set `self.Open` false)
  (goto _label))

(fn `UserConstructionScript`
  (set `self.LeftClosedLocation` (`SceneComponent.RelativeLocation` (`self.LeftDoor`)))
  (set `self.RightClosedLocation` (`SceneComponent.RelativeLocation` (`self.RightDoor`))))