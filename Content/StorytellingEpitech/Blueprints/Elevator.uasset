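; Elevator actor whose platform moves between its starting position and a travel point when triggered.
; It implements a Triggerable interface that sets or clears a Triggered flag.
; Each Tick moves the platform at constant speed toward the travel point while triggered, or back to the original position otherwise.
; The construction script records that original relative location, and movement is done without sweep.
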(event `self.ReceiveTick`
  (params (DeltaSeconds :type "Float (single-precision)"))
  (`SceneComponent.K2_SetRelativeLocation` (`self.Platform`) (`KismetMathLibrary.VInterpTo_Constant` (`SceneComponent.RelativeLocation` (`self.Platform`)) (`KismetMathLibrary.SelectVector` (`SceneComponent.RelativeLocation` (`self.TravelPoint`)) (`self.OriginalPosition`) (`self.Triggered`)) DeltaSeconds (`self.PlatformSpeed`)) false false))

(event `self.Triggerable.OnTrigger`
  (params (Instigator :type "Actor Object Reference") (`Instigator Component` :type "ActorComponent Object Reference"))
  (set `self.Triggered` true))

(event `self.Triggerable.OnUntrigger`
  (params (Instigator :type "Actor Object Reference") (`Instigator Component` :type "ActorComponent Object Reference"))
  (set `self.Triggered` false))

(fn `UserConstructionScript`
  (set `self.OriginalPosition` (`SceneComponent.RelativeLocation` (`self.Platform`))))