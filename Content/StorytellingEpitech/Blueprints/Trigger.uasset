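; Trigger component that relays trigger and untrigger signals from its owning actor to a list of target actors.
; Trigger and Untrigger loop over TriggeredActors, find each actor's Triggerable component and call the matching function on it.
; The owner is passed as instigator and this component as instigator component, and targets lacking a Triggerable are skipped.
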(fn `Trigger`
  (for _array_element (`self.TriggeredActors`)
    (bind _returnvalue (`Actor.GetComponentByClass` _array_element "/Game/StorytellingEpitech/Blueprints/Triggerable.Triggerable_C"))
    (`/Engine/EditorBlueprintResources/StandardMacros.IsValid` _returnvalue
      (:`Is Valid`
        (`/Game/StorytellingEpitech/Blueprints/Triggerable.Trigger` _returnvalue (`self.GetOwner`) self)))))

(fn `Untrigger`
  (for _array_element (`self.TriggeredActors`)
    (bind _returnvalue (`Actor.GetComponentByClass` _array_element "/Game/StorytellingEpitech/Blueprints/Triggerable.Triggerable_C"))
    (`/Engine/EditorBlueprintResources/StandardMacros.IsValid` _returnvalue
      (:`Is Valid`
        (`/Game/StorytellingEpitech/Blueprints/Triggerable.Untrigger` _returnvalue (`self.GetOwner`) self)))))