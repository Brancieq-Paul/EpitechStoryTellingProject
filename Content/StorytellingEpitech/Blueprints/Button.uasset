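; Pressure-plate style button actor that drives a Trigger component when something stands on it.
; The first overlap with Cube1 fires the trigger, plays a click sound and swaps the cube to its pressed material.
; When Cube1's last overlapping actor leaves, it untriggers and restores the default material, so extra occupants do not re-fire it.
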(event `self.ReceiveActorBeginOverlap`
  (params (OtherActor :type "Actor Object Reference"))
  (if (== (`KismetArrayLibrary.Array_Length` (`PrimitiveComponent.GetOverlappingActors` (`self.Cube1`) null)) 1)
    (`/Game/StorytellingEpitech/Blueprints/Trigger.Trigger` (`self.Trigger`))
    (`GameplayStatics.PlaySound2D` "/Game/ThirdPerson/Sounds/mixkit-classic-click-1117.mixkit-classic-click-1117" 1.0 1.0 0.0 null null)
    (`PrimitiveComponent.SetMaterial` (`self.Cube1`) 0 "/Game/StorytellingEpitech/Materials/ButtonMaterial_2.ButtonMaterial_2")))

(event `self.ReceiveActorEndOverlap`
  (params (OtherActor :type "Actor Object Reference"))
  (if (`KismetArrayLibrary.Array_IsEmpty` (`PrimitiveComponent.GetOverlappingActors` (`self.Cube1`) null))
    (`/Game/StorytellingEpitech/Blueprints/Trigger.Untrigger` (`self.Trigger`))
    (`PrimitiveComponent.SetMaterial` (`self.Cube1`) 0 "/Game/StorytellingEpitech/Materials/ButtonMaterial.ButtonMaterial")))

(fn `UserConstructionScript`)